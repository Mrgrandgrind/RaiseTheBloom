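; ValveBP is a placeholder valve Blueprint for the submarine, kept in the BrokenThingsIShouldntDelete folder.
; It stubs an interaction interface covering hover, drag, pickup and use, with every handler returning false.
; Its closest-point query returns a zero vector and zero priority.
; The event graph and construction script are empty, so it has no scripted behavior.
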(event EventBeginPlay)

(event Collision|EventActorBeginOverlap
  (params (OtherActor :type Actor%20Object%20Reference)))

(event EventTick
  (params (DeltaSeconds :type Float%20%28single-precision%29)))

(fn ConstructionScript)

(fn GetClosestPointandPriority
  (params (Interactor :type BPC%20World%20Interactor%20Object%20Reference))
  (return "0, 0, 0" 0))

(fn OnDrag
  (params (Interactor :type BPC%20World%20Interactor%20Object%20Reference))
  (return false))

(fn OnDragStart
  (params (Interactor :type BPC%20World%20Interactor%20Object%20Reference))
  (return false))

(fn OnDragStop
  (params (Interactor :type BPC%20World%20Interactor%20Object%20Reference))
  (return false))

(fn OnHover
  (params (Interactor :type BPC%20World%20Interactor%20Object%20Reference))
  (return false))

(fn OnPickupPressed
  (params (Interactor :type BPC%20World%20Interactor%20Object%20Reference))
  (return false))

(fn OnPickupReleased
  (params (Interactor :type BPC%20World%20Interactor%20Object%20Reference))
  (return false))

(fn OnUnhover
  (params (Interactor :type BPC%20World%20Interactor%20Object%20Reference))
  (return false))

(fn OnUsePressed
  (params (Interactor :type BPC%20World%20Interactor%20Object%20Reference))
  (return false))

(fn OnUseReleased
  (params (Interactor :type BPC%20World%20Interactor%20Object%20Reference))
  (return false))